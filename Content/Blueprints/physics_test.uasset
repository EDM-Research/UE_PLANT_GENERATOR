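; Physics test Blueprint that repeatedly spawns procedural grape variations high above the world origin, with random pitch and roll.
; On BeginPlay, a delayed loop calls CreateVariation with physics enabled, a grape detach chance and an "ispurple" parameter fed by Color.
; Color is bitwise-inverted between spawns.
; The NumCrops counter is clamped with Min rather than decremented, so the loop never reaches its zero exit.
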(event `self.ReceiveBeginPlay`
  (set `self.NumCrops` 10)
  (`Crop_Generator.Create_variation` "Grape" (`KismetMathLibrary.MakeTransform` (`KismetMathLibrary.MakeVector` 0.0 0.0 3000.0) (`KismetMathLibrary.MakeRotator` (`KismetMathLibrary.Conv_IntToDouble` (`KismetMathLibrary.RandomIntegerInRange` -90 90)) (`KismetMathLibrary.Conv_IntToDouble` (`KismetMathLibrary.RandomIntegerInRange` -90 90)))) (`|MakeMap` "ispurple" (`KismetMathLibrary.Conv_IntToDouble` (stale _output_get_2)) "PhysicsEnabled" 1.0 "GrapeDetachChance" 0.2 :!valuetype "Float (single-precision)") :!label _label)
  (`KismetSystemLibrary.Delay` 3.0)
  (bind _output_get (set `self.NumCrops` (`KismetMathLibrary.Min` (`self.NumCrops`) 1)))
  (if (not (== _output_get 0))
    (bind _output_get_2 (set `self.Color` (`KismetMathLibrary.Not_Int` (`self.Color`))))
    (goto _label)))

(fn `UserConstructionScript`)