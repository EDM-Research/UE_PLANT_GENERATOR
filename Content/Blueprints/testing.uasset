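; Test Blueprint that stress-spawns procedural apple variations when play begins.
; BeginPlay loops a thousand times, calling CreateVariation with the Apple generator type and an "isred" parameter set to zero.
; Modulo and integer division on the loop index lay the apples out in a tightly spaced grid, ten columns wide, at a fixed height.
; The construction script is empty.
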(event `self.ReceiveBeginPlay`
  (bind _returnvalue (`KismetMathLibrary.Conv_Int64ToInt` 10))
  (for _index (range 1000)
    (`Crop_Generator.Create_variation` "Apple" (`KismetMathLibrary.MakeTransform` (`KismetMathLibrary.MakeVector` (`KismetMathLibrary.Conv_IntToDouble` (* (mod _index 10) _returnvalue)) (`KismetMathLibrary.Conv_IntToDouble` (* (/ _index 10) _returnvalue)) 10.0)) (`|MakeMap` "isred" 0.0 :!valuetype "Float (single-precision)"))))

(fn `UserConstructionScript`)